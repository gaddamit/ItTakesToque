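; Co-op Game Mode that adds a second local player when play begins and sends a Mage character switcher at that player's pawn.
; BeginPlay creates the player, casts its pawn to BP_Character and spawns BP_CharacterSwitcher_Mage below the character's mesh as Hat.
; Tick nudges Hat upward each frame, sweeping off, so it rises through the character until a short delay destroys it.
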(event EventBeginPlay
  (bind _returnvalue (Class|GameplayStatics|CreatePlayer -1))
  (bind _asbp_character (Utilities|Casting|CastToBP_Character (Pawn|GetControlledPawn _returnvalue)))
  (bind _returnvalue_2 (Game|SpawnActorfromClass "/Game/Blueprints/Collectibles/BP_CharacterSwitcher_Mage.BP_CharacterSwitcher_Mage_C" (Math|Transform|MakeTransform (+ (.location (Transformation|GetWorldTransform (Variables|/Script/Engine.Character|GetMesh _asbp_character))) "0.000000,0.000000,-100.000000") "0, 0, 0" "1.000000,1.000000,1.000000") "Undefined" "MultiplyWithRoot" 0 0))
  (bind _output_get (Variables|Default|SetHat _returnvalue_2))
  (Utilities|FlowControl|Delay 0.5)
  (Actor|DestroyActor _output_get))

(event EventTick
  (params (DeltaSeconds :type Float%20%28single-precision%29))
  (bind _hat (Variables|Default|GetHat))
  (Utilities|IsValid _hat
    (:Is%20Valid
      (Transformation|AddActorWorldOffset _hat "0.000000,0.000000,5.000000"))))

(fn ConstructionScript)