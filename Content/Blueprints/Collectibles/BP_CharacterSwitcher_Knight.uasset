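; BP_CharacterSwitcher_Knight is the Knight variant of a character-switcher collectible, supplying its idle motion and overlap feedback.
; On BeginPlay, its tilted mesh bobs up and down endlessly through two eased MoveComponentTo moves looped back on themselves.
; OverlapEffects turns an overlapping BP_Character's Niagara indicator ring white, then spawns a white poof at the mesh when that indicator is valid.
; The switch logic itself is absent from these graphs.
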(event EventBeginPlay
  (Components|MoveComponentTo (Variables|Default|GetStaticMesh) "0.000000,0.000000,25.000000" "0.000000,-45.000000,-20.000000" true true 2.0 false :!label _label)
  (Components|MoveComponentTo (Variables|Default|GetStaticMesh) "0.000000,0.000000,-25.000000" "0.000000,-45.000000,-20.000000" true true 2.0 false)
  (goto _label))

(event EventOverlapEffects
  (params (OtherActor :type Actor%20Object%20Reference))
  (bind _linearcolor (Utilities|Struct|MakeLinearColor 1.0 1.0 1.0 1.0))
  (bind _asbp_character (Utilities|Casting|CastToBP_Character OtherActor))
  (Utilities|IsValid (Variables|/Game/Blueprints/BP_Character.BP_Character_C|GetIndicator _asbp_character)
    (:Is%20Valid
      (Niagara|SetNiagaraVariable(LinearColor) (Variables|/Game/Blueprints/BP_Character.BP_Character_C|GetIndicator _asbp_character) (Utilities|String|MakeLiteralString "User.Ring Color") _linearcolor)
      (bind _returnvalue (Niagara|SpawnSystematLocation "/Game/Effects/P_Poof.P_Poof" (Transformation|GetWorldLocation (Variables|Default|GetStaticMesh))))
      (Niagara|SetNiagaraVariable(LinearColor) _returnvalue "ColorStart" _linearcolor))))

(fn ConstructionScript)