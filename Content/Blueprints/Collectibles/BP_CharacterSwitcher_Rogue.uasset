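; Collectible character switcher for the Rogue, judging by its name, with a floating mesh and an empty OverlapEffects event.
; On BeginPlay it looks up CharacterColor by CharacterType in the SCharacterColors map, then endlessly eases the tilted mesh up and down with chained MoveComponentTo calls.
; Unreachable leftover logic would tint the character's Niagara indicator ring and spawn a matching poof effect in a hardcoded color.
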(event EventBeginPlay
  (Variables|Default|SetCharacterColor (.Value (Utilities|Map|Find (.colors (Utilities|Struct|MakeS_CharacterColors "((KNIGHT, (R=1.000000,G=1.000000,B=1.000000,A=1.000000)),(BARBARIAN, (R=8.000000,G=5.000000,B=0.100000,A=1.000000)),(ROGUE, (R=8.000000,G=0.080000,B=0.200000,A=1.000000)),(MAGE, (R=1.000000,G=0.300000,B=8.000000,A=1.000000)),(NONE, (R=0.000000,G=0.000000,B=0.000000,A=0.000000)))")) (Variables|Default|GetCharacterType))))
  (Components|MoveComponentTo (Variables|Default|GetStaticMesh) "0.000000,0.000000,25.000000" "0.000000,-45.000000,-20.000000" true true 2.0 false :!label _label)
  (Components|MoveComponentTo (Variables|Default|GetStaticMesh) "0.000000,0.000000,-25.000000" "0.000000,-45.000000,-20.000000" true true 2.0 false)
  (goto _label))

(event EventOverlapEffects
  (params (OtherActor :type Actor%20Object%20Reference)))

(fn ConstructionScript)