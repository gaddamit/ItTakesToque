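; Spawner actor that periodically drops random actors from a configurable class list around itself.
; A timer set at BeginPlay, optionally looping, fires after each interval; following a short delay it spawns a set amount if enabled.
; Each spawn uses a random reachable navmesh point within a radius derived from a component's scale, raised slightly and collision-adjusted.
; An Enable function switches spawning on or off.
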(event Custom|SpawnActors
  (bind _actorstospawn (Variables|Default|GetActorsToSpawn))
  (Utilities|FlowControl|Delay 0.2)
  (if (Variables|Default|GetEnabled)
    (for _index (range 0 (- (Variables|Default|GetAmount) 1))
      (Game|SpawnActorfromClass (Utilities|Array|Get(acopy) _actorstospawn (Math|Random|RandomInteger (Utilities|Array|Length _actorstospawn))) (Math|Transform|MakeTransform (+ (.RandomLocation (AI|Navigation|GetRandomReachablePointinRadius (.location (Transformation|GetWorldTransform (Variables|Default|GetSphere))) (* (.x (Transformation|GetWorldScale (Variables|Default|GetRadius))) 5e+01) 0 0)) "0.000000,0.000000,100.000000") "0, 0, 0" "1.000000,1.000000,1.000000") "AdjustIfPossibleButAlwaysSpawn" "MultiplyWithRoot" 0 0))))

(event EventBeginPlay
  (Utilities|Time|SetTimerbyEvent (delegate Custom|SpawnActors) (Variables|Default|GetInterval) (Variables|Default|GetLooping)))

(fn ConstructionScript)

(fn Enable
  (params (Value :type Boolean))
  (Variables|Default|SetEnabled Value))