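; Gameplay Ability that gives the avatar a short, fast forward dash.
; It applies a constant root motion force along the actor's forward vector, then restores the velocity captured at activation.
; It flags IsDashing on the character's ABP_Character anim instance during the dash.
; On finish it commits the cooldown again after the initial CommitAbility, ends the ability and clears the flag.
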(event Ability|EventActivateAbility
  (bind _returnvalue (Ability|GetAvatarActorfromActorInfo))
  (Ability|CommitAbility)
  (Ability|Tasks|ApplyRootMotionConstantForce "None" (Transformation|GetActorForwardVector _returnvalue) 3e+03 0.1 false 0 "SetVelocity" (Transformation|GetVelocity _returnvalue)
    (:then
      (bind _asbp_character (Utilities|Casting|CastToBP_Character (Ability|GetAvatarActorfromActorInfo)))
      (bind _asabp_character (Utilities|Casting|CastToABP_Character (Components|SkeletalMesh|GetAnimInstance (Variables|/Script/Engine.Character|GetMesh _asbp_character))))
      (Variables|/Game/Blueprints/ABPS/ABP_Character.ABP_Character_C|SetIsDashing _asabp_character true))
    (:OnFinish
      (Ability|CommitAbilityCooldown false)
      (Ability|EndAbility)
      (Variables|/Game/Blueprints/ABPS/ABP_Character.ABP_Character_C|SetIsDashing _asabp_character false))))

(event Ability|EventOnEndAbility
  (params (bWasCancelled :type Boolean)))