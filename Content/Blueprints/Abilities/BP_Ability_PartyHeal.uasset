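; Gameplay ability that heals the party by applying GE_PartyHeal to every player-controlled BP_Character.
; On activation it commits, plays the skill montage and waits for an Ability.BasicSpell gameplay event.
; When the event arrives, it loops over the player controllers and each character's own ability system applies the effect to itself, then the ability ends.
; Only that event path calls EndAbility; montage interruption or cancellation is not handled.
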(event Ability|EventActivateAbility
  (Ability|CommitAbility)
  (|PlayMontageandWaitProxy "None" (Variables|Default|GetSkillAnimation) 1.0 "None" true 1.0 0.0 false
    (:then
      (Ability|Tasks|WaitGameplayEvent "(TagName=\"Ability.BasicSpell\")" 0
        (:EventReceived
          (for _index (range 0 (- (Class|GameplayStatics|GetNumPlayerControllers) 1))
            (bind _asbp_character (Utilities|Casting|CastToBP_Character (Pawn|GetControlledPawn (Game|GetPlayerController _index))))
            (GameplayEffects|ApplyGameplayEffectToTarget :self (Variables|/Game/Blueprints/Characters/BP_Character.BP_Character_C|GetMy2AbilitySystem _asbp_character) :GameplayEffectClass "/Game/Blueprints/Effects/GE_PartyHeal.GE_PartyHeal_C" :Target (Variables|/Game/Blueprints/Characters/BP_Character.BP_Character_C|GetMy2AbilitySystem _asbp_character)))
          (Ability|EndAbility))))))

(event Ability|EventOnEndAbility
  (params (bWasCancelled :type Boolean)))