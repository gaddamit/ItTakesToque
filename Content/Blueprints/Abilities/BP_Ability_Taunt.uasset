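; BP_Ability_Taunt is a gameplay ability that makes every BP_Character_Enemy_Base actor in the world target the caster.
; It commits, plays a skill montage and waits for the Ability.BasicSpell gameplay event.
; On that event it writes the owner into each enemy's AttackTarget blackboard key and applies GE_Taunt to those enemies and the owner.
; Only montage completion ends the ability; other montage outcomes are unhandled.
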(event Ability|EventActivateAbility
  (Ability|CommitAbility)
  (|PlayMontageandWaitProxy "None" (Variables|Default|GetSkillAnimation) 1.0 "None" true 1.0 0.0 false
    (:then
      (Ability|Tasks|WaitGameplayEvent "(TagName=\"Ability.BasicSpell\")" 0
        (:EventReceived
          (bind _outactors (Actor|GetAllActorsOfClass "/Game/Blueprints/Characters/Enemies/BP_Character_Enemy_Base.BP_Character_Enemy_Base_C"))
          (for _array_element _outactors
            (CallFunction|ChangeAttackTarget _array_element (Ability|GetOwningActorfromActorInfo self))
            (GameplayEffects|ApplyGameplayEffectToSelf :self (Variables|/Game/Blueprints/Characters/BP_Character.BP_Character_C|GetMy2AbilitySystem _array_element) :GameplayEffectClass "/Game/Blueprints/Effects/GE_Taunt.GE_Taunt_C"))
          (Ability|ApplyGameplayEffectToOwner "/Game/Blueprints/Effects/GE_Taunt.GE_Taunt_C"))))
    (:OnCompleted
      (Ability|EndAbility))))

(event Ability|EventOnEndAbility
  (params (bWasCancelled :type Boolean)))

(fn ChangeAttackTarget
  (params (EnemyAI :type BP%20Character%20Enemy%20Base%20Object%20Reference) (NewTarget :type Actor%20Object%20Reference))
  (AI|Components|Blackboard|SetValueasObject (AI|GetBlackboard EnemyAI) (Utilities|Name|MakeLiteralName "AttackTarget") NewTarget))