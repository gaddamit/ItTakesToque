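; Gameplay ability for a basic melee combo that slows the character's walk speed while active.
; It plays the current combo montage, waiting on gameplay events for the combo window and for melee hits, which apply the damage effect to the event's targets.
; An open window advances the combo index so another input plays the next montage.
; Montage completion ends the ability, and ending resets combo state and speed.
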(event Ability|EventActivateAbility
  (Ability|CommitAbility)
  (bind _asbp_character (Utilities|Casting|CastToBP_Character (Ability|GetOwningActorfromActorInfo)))
  (Variables|/Script/Engine.CharacterMovementComponent|SetMaxWalkSpeed (Variables|/Script/Engine.Character|GetCharacterMovement _asbp_character) 1e+02)
  (|PlayMontageandWaitProxy "None" (Utilities|Array|Get(acopy) (Variables|Default|GetMontages) (Variables|Default|GetCurrentCombo)) 1.5 "None" true 1.0 0.0 false
    (:then
      (Ability|Tasks|WaitGameplayEvent "(TagName=\"Event.ComboWindowOpen\")" 0 true
        (:then
          (bind _payload (Ability|Tasks|WaitGameplayEvent "(TagName=\"Damage.Melee\")" 0)
            (:EventReceived
              (GameplayEffects|ApplyGameplayEffectToTarget (.TargetData (Utilities|Struct|BreakGameplayEventData _payload)) "/Game/Blueprints/Effects/GE_Damage.GE_Damage_C" 1 1))))
        (:EventReceived
          (Variables|Default|SetCanCombo true)
          (Math|Integer|IncrementInt (Variables|Default|GetCurrentCombo)))))
    (:OnCompleted
      (Ability|EndAbility))))

(event Ability|EventOnEndAbility
  (params (bWasCancelled :type Boolean))
  (Variables|Default|SetCurrentCombo 0)
  (Variables|Default|SetCanCombo false)
  (bind _asbp_character (Utilities|Casting|CastToBP_Character (Ability|GetOwningActorfromActorInfo)))
  (Variables|/Script/Engine.CharacterMovementComponent|SetMaxWalkSpeed (Variables|/Script/Engine.Character|GetCharacterMovement _asbp_character) 1e+03))

(event EventOnInputPressed
  (if (Variables|Default|GetCanCombo)
    (Variables|Default|SetCanCombo false)
    (|PlayMontageandWaitProxy "None" (Utilities|Array|Get(acopy) (Variables|Default|GetMontages) (Variables|Default|GetCurrentCombo)) 1.5 "None" true 1.0 0.0 false
      (:then
        (Ability|Tasks|WaitGameplayEvent "(TagName=\"Event.ComboWindowOpen\")" 0 true
          (:then
            (bind _payload (Ability|Tasks|WaitGameplayEvent "(TagName=\"Damage.Melee\")" 0)
              (:EventReceived
                (GameplayEffects|ApplyGameplayEffectToTarget (.TargetData (Utilities|Struct|BreakGameplayEventData _payload)) "/Game/Blueprints/Effects/GE_Damage.GE_Damage_C" 1 1))))
          (:EventReceived
            (Variables|Default|SetCanCombo true)
            (Math|Integer|IncrementInt (Variables|Default|GetCurrentCombo)))))
      (:OnCompleted
        (Ability|EndAbility)))))