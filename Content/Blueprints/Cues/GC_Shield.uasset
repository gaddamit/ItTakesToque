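; Gameplay cue for a shield effect, which attaches a Niagara system to the mesh of the target BP_Character.
; OnExecute prints a debug string and spawns the system, while OnActive spawns it and greatly enlarges its world scale.
; Both spawns rely on auto-destroy, as the cue keeps no reference and defines no removal handler.
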(fn OnExecute
  (params (MyTarget :type Actor%20Object%20Reference) (Parameters :type Gameplay%20Cue%20Parameters%20Structure%20%28by%20ref%29))
  (Development|PrintString 0)
  (bind _asbp_character (Utilities|Casting|CastToBP_Character MyTarget))
  (Niagara|SpawnSystemAttached (Variables|Default|GetSystem%20Template) (Variables|/Script/Engine.Character|GetMesh _asbp_character) "None" "0, 0, 0" "0, 0, 0" "KeepRelativeOffset" true)
  (return true))

(fn OnActive
  (params (MyTarget :type Actor%20Object%20Reference) (Parameters :type Gameplay%20Cue%20Parameters%20Structure%20%28by%20ref%29))
  (bind _asbp_character (Utilities|Casting|CastToBP_Character MyTarget))
  (bind _returnvalue (Niagara|SpawnSystemAttached (Variables|Default|GetSystem%20Template) (Variables|/Script/Engine.Character|GetMesh _asbp_character) "None" "0, 0, 0" "0, 0, 0" "KeepRelativeOffset" true))
  (Transformation|SetWorldScale3D _returnvalue "30.000000,30.000000,30.000000")
  (return true))