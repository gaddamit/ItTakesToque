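; Gameplay Cue that freezes enemy characters in place while it is active.
; OnActive casts the target to BP_Character_Enemy_Base and disables ticking on its Mesh and CharacterMovement components, halting animation and movement updates.
; OnRemove re-enables both ticks, while OnExecute only prints a placeholder debug string.
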(fn OnExecute
  (params (MyTarget :type Actor%20Object%20Reference) (Parameters :type Gameplay%20Cue%20Parameters%20Structure%20%28by%20ref%29))
  (Development|PrintString 0)
  (return false))

(fn OnActive
  (params (MyTarget :type Actor%20Object%20Reference) (Parameters :type Gameplay%20Cue%20Parameters%20Structure%20%28by%20ref%29))
  (bind _asbp_character_enemy_base (Utilities|Casting|CastToBP_Character_Enemy_Base MyTarget))
  (Components|Tick|SetComponentTickEnabled (Variables|/Script/Engine.Character|GetMesh _asbp_character_enemy_base) false)
  (Components|Tick|SetComponentTickEnabled (Variables|/Script/Engine.Character|GetCharacterMovement _asbp_character_enemy_base) false)
  (return true))

(fn OnRemove
  (params (MyTarget :type Actor%20Object%20Reference) (Parameters :type Gameplay%20Cue%20Parameters%20Structure%20%28by%20ref%29))
  (bind _asbp_character_enemy_base (Utilities|Casting|CastToBP_Character_Enemy_Base MyTarget))
  (Components|Tick|SetComponentTickEnabled (Variables|/Script/Engine.Character|GetMesh _asbp_character_enemy_base) true)
  (Components|Tick|SetComponentTickEnabled (Variables|/Script/Engine.Character|GetCharacterMovement _asbp_character_enemy_base) true)
  (return true))