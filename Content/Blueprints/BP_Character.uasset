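; BP_Character is a character Blueprint for a co-op game, handling GAS-driven melee hits and death, and removing the indicator on undead types.
; TraceWeaponPath sphere-traces along equipped weapons and sends throttled Damage.Melee gameplay events to itself, with hit characters as targets.
; OnDamageReceived checks an ability-system attribute; on death it disables input, plays a montage, requests a GM_CoOp respawn, then destroys weapons and character.
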(event EventBeginPlay
  (if (Utilities|Enum|Equal(Enum) (Variables|Default|GetCharacterType) "UNDEAD")
    (Components|DestroyComponent (Variables|Default|GetIndicator))))

(event EventOnDamageReceived
  (if (Variables|Default|GetIsStillAlive)
    (bind _isalive (CallFunction|IsAlive))
    (bind _output_get (Variables|Default|SetIsStillAlive _isalive))
    (if (not _output_get)
      (Input|DisableInput 0)
      (bind _returnvalue (Animation|PlayAnimMontage (select (Variables|Default|GetIsStillAlive) (Variables|Default|GetAnimationOnHit) (Variables|Default|GetAnimationOnDeath)) 1.0 "None"))
      (if (not (Variables|Default|GetIsStillAlive))
        (Utilities|FlowControl|Delay _returnvalue)
        (bind _asgm_co_op (Utilities|Casting|CastToGM_CoOp (Game|GetGameMode)))
        (bind _asplayer_controller (Utilities|Casting|CastToPlayerController (Pawn|GetController self)))
        (Default|RespawnPlayer _asgm_co_op _asplayer_controller)
        (CallFunction|DestroyAfterDelay)))))

(event EventTraceWeaponPath
  (bind _characterweapons1 (Variables|Default|GetCharacterWeapons1))
  (Utilities|Array|Clear (Variables|Default|GetTargetActors))
  (Utilities|IsValid _characterweapons1
    (:Is%20Valid
      (bind _values (Utilities|Map|Values (Variables|/Script/ItTakesToque.CharacterWeapons|GetEquippedWeapons _characterweapons1)))
      (for _array_element _values
        (bind (_outhits _returnvalue) (Collision|MultiSphereTraceForObjects (Transformation|GetWorldLocation (Variables|/Script/ItTakesToque.Weapon|GetStart _array_element)) (Transformation|GetWorldLocation (Variables|/Script/ItTakesToque.Weapon|GetEnd _array_element)) 1e+02 (Utilities|Array|MakeArray "ObjectTypeQuery8") false 0 "ForOneFrame"))
        (if _returnvalue
          (for _array_element_2 _outhits
            (Utilities|Array|AddUnique (Variables|Default|GetTargetActors) (.HitActor (Collision|BreakHitResult _array_element_2))))
          (Utilities|FlowControl|DoOnce false :!label _label
            (:Completed
              (CallFunction|SendDamageEventtoTargets (Variables|Default|GetTargetActors))
              (Utilities|FlowControl|Delay 0.5)
              (goto _label Reset))))))))

(fn ConstructionScript)

(fn SendDamageEventtoTargets
  (params (Actors :type Array%20of%20Actor%20Object%20References))
  (bind _self self)
  (for _array_element Actors
    (bind _asbp_character (Utilities|Casting|CastToBP_Character _array_element))
    (Ability|SendGameplayEventtoActor _self "(TagName=\"Damage.Melee\")" (Utilities|Struct|MakeGameplayEventData "(TagName=\"\")" _self _asbp_character 0 0 "()" (GameplayTags|GetOwnedGameplayTags 0 :!class /Script/GameplayTags.BlueprintGameplayTagLibrary) (GameplayTags|GetOwnedGameplayTags _asbp_character :!class /Script/GameplayTags.BlueprintGameplayTagLibrary) 0.0 (Ability|TargetData|AbilityTargetDatafromActor _asbp_character)))))

(fn DestroyAfterDelay
  (bind _characterweapons1 (Variables|Default|GetCharacterWeapons1))
  (Utilities|IsValid _characterweapons1
    (:Is%20Valid
      (bind _values (Utilities|Map|Values (Variables|/Script/ItTakesToque.CharacterWeapons|GetEquippedWeapons _characterweapons1)))
      (for _array_element _values
        (Actor|DestroyActor _array_element))
      (Actor|DestroyActor))))

(fn IsAlive
  (bind _my2abilitysystem (Variables|Default|GetMy2AbilitySystem))
  (bind (_bfound _returnvalue) (Class|AbilitySystemComponent|GetGameplayAttributeValue _my2abilitysystem "(AttributeName=\"Health\",Attribute=/Script/ItTakesToque.CharacterAttributeSet:Health,AttributeOwner=\"/Script/CoreUObject.Class'/Script/ItTakesToque.CharacterAttributeSet'\")"))
  (if _bfound
    (return (> _returnvalue 0.0))
    (else
      (return false))))