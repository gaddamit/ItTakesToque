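; BP_LevelActivator is a level actor that starts the level once two different BP_Character actors meet inside its sphere.
; On BeginPlay it caches the level's BP_Gate and all BP_ActorSpawner actors.
; The first character to overlap is stored, and a different one entering sets IsActivated, activates the gate and enables every spawner.
; Any end overlap clears the stored character, regardless of which actor left.
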(event OnComponentBeginOverlap(Sphere)
  (params (OverlappedComponent :type Primitive%20Component%20Object%20Reference) (OtherActor :type Actor%20Object%20Reference) (OtherComp :type Primitive%20Component%20Object%20Reference) (OtherBodyIndex :type Integer) (bFromSweep :type Boolean) (SweepResult :type Hit%20Result%20Structure%20%28by%20ref%29))
  (if (Variables|Default|GetIsActivated)
    _
    (else
      _))
  (bind _asbp_character (Utilities|Casting|CastToBP_Character OtherActor))
  (Utilities|IsValid (Variables|Default|GetCharacter)
    (:Is%20Valid
      (if (!= (Variables|Default|GetCharacter) _asbp_character)
        (Variables|Default|SetIsActivated true)
        (Default|Activate (Variables|Default|GetGate))
        (for _array_element (Variables|Default|GetSpawners)
          (Variables|/Game/Blueprints/LevelActors/BP_ActorSpawner.BP_ActorSpawner_C|SetEnabled _array_element true))))
    (:Is%20Not%20Valid
      (Variables|Default|SetCharacter _asbp_character))))

(event OnComponentEndOverlap(Sphere)
  (params (OverlappedComponent :type Primitive%20Component%20Object%20Reference) (OtherActor :type Actor%20Object%20Reference) (OtherComp :type Primitive%20Component%20Object%20Reference) (OtherBodyIndex :type Integer))
  (Variables|Default|SetCharacter 0))

(event EventBeginPlay
  (bind _returnvalue (Actor|GetActorOfClass "/Game/Blueprints/LevelActors/BP_Gate.BP_Gate_C"))
  (Variables|Default|SetGate _returnvalue)
  (bind _outactors (Actor|GetAllActorsOfClass "/Game/Blueprints/LevelActors/BP_ActorSpawner.BP_ActorSpawner_C"))
  (Variables|Default|SetSpawners _outactors))

(fn ConstructionScript)