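; BP_LevelGate is a level gate actor that, on activation, can spawn character switcher actors for the co-op game.
; If ShouldSpawnCollectibles is set, OnActivate asks GI_CoOp for the free character types and maps each to its Knight, Barbarian, Rogue or Mage switcher class.
; Switchers spawn raised above the gate, with the X offset flipping sign after each spawn to alternate between two sides.
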(event EventBeginPlay)

(event Collision|EventActorBeginOverlap
  (params (OtherActor :type Actor%20Object%20Reference)))

(event EventTick
  (params (DeltaSeconds :type Float%20%28single-precision%29)))

(event EventOnActivate
  (bind _returnvalue (Transformation|GetActorTransform))
  (if (Variables|Default|GetShouldSpawnCollectibles)
    (bind _asgi_co_op (Utilities|Casting|CastToGI_CoOp (Game|GetGameInstance)))
    (bind _freecharactertypes (Default|GetFreeCharacterTypes _asgi_co_op))
    (for _array_element _freecharactertypes
      (Game|SpawnActorfromClass (Utilities|Select :Index _array_element :NONE 0 :KNIGHT "/Game/Blueprints/Collectibles/BP_CharacterSwitcher_Knight.BP_CharacterSwitcher_Knight_C" :BARBARIAN "/Game/Blueprints/Collectibles/BP_CharacterSwitcher_Barbarian.BP_CharacterSwitcher_Barbarian_C" :ROGUE "/Game/Blueprints/Collectibles/BP_CharacterSwitcher_Rogue.BP_CharacterSwitcher_Rogue_C" :MAGE "/Game/Blueprints/Collectibles/BP_CharacterSwitcher_Mage.BP_CharacterSwitcher_Mage_C" :UNDEAD 0) (Math|Transform|MakeTransform (Math|Vector|MakeVector (+ (.x (.location _returnvalue)) (Variables|Default|GetLocationStarting)) (.y (.location _returnvalue)) (+ (.z (.location _returnvalue)) 1e+02)) "0, 0, 0" "1.000000,1.000000,1.000000") "Undefined" "MultiplyWithRoot" 0 0)
      (Variables|Default|SetLocationStarting (* (Variables|Default|GetLocationStarting) -1.0)))))

(fn ConstructionScript)