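; Base enemy character Blueprint that passes its Behavior Tree to the enemy AI controller on possession and removes its spotlight at BeginPlay.
; Weapon attacks sphere-trace along each equipped weapon and apply a GAS damage effect to hit characters, throttled by a DoOnce with a delayed reset.
; Received damage plays a hit montage or starts death, which disables movement, plays the death montage, then unpossesses to destroy the actor.
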(event EventBeginPlay
  (|CallParentFunction)
  (Components|DestroyComponent (Variables|Default|GetSpotLight)))

(event EventPossessed
  (params (NewController :type Controller%20Object%20Reference))
  (bind _self self)
  (bind _returnvalue (AI|GetAIController _self))
  (Utilities|IsValid _returnvalue
    (:Is%20Valid
      (bind _asaic_enemy_base (Utilities|Casting|CastToAIC_Enemy_Base _returnvalue))
      (Variables|/Game/AI/AIC_Enemy_Base.AIC_Enemy_Base_C|SetBTAsset _asaic_enemy_base (Variables|Default|GetBehaviorTree)))))

(event EventOnDamageReceived
  (if (and (Variables|Default|GetbHasSpawned) (Variables|Default|GetbIsAlive))
    (bind _isalive (CallFunction|IsAlive))
    (bind _output_get (Variables|Default|SetbIsAlive _isalive))
    (if _output_get
      (Animation|PlayAnimMontage (Variables|Default|GetAnimationOnHit) 1.0 "None")
      (else
        (CallFunction|StartDeath)))))

(event Collision|EventActorBeginOverlap
  (params (OtherActor :type Actor%20Object%20Reference))
  (|CallParentFunction OtherActor) ; This node is disabled and will not be called.\nDrag off pins to build functionality.
)

(event EventTick
  (params (DeltaSeconds :type Float%20%28single-precision%29))
  (|CallParentFunction DeltaSeconds) ; This node is disabled and will not be called.\nDrag off pins to build functionality.
)

(event EventStartDeath
  (Pawn|Components|CharacterMovement|DisableMovement (Variables|Character|GetCharacterMovement))
  (bind _returnvalue (Animation|PlayAnimMontage (Variables|Default|GetAnimationOnDeath) 1.0 "None"))
  (Utilities|FlowControl|Delay (+ _returnvalue 1.0))
  (Pawn|UnPossess (Pawn|GetController)))

(event EventUnpossessed
  (params (OldController :type Controller%20Object%20Reference))
  (CallFunction|DestroyActorandComponents))

(event EventDestroyed)

(event EventTraceWeaponPath
  (bind _characterweapons1 (Variables|Default|GetCharacterWeapons1))
  (Utilities|Array|Clear (Variables|Default|GetTargetActors))
  (Utilities|IsValid _characterweapons1
    (:Is%20Valid
      (bind _values (Utilities|Map|Values (Variables|/Script/ItTakesToque.CharacterWeapons|GetEquippedWeapons _characterweapons1)))
      (for _array_element _values
        (bind (_outhits _returnvalue) (Collision|MultiSphereTraceForObjects (Transformation|GetWorldLocation (Variables|/Script/ItTakesToque.Weapon|GetStart _array_element)) (Transformation|GetWorldLocation (Variables|/Script/ItTakesToque.Weapon|GetEnd _array_element)) 5e+01 (Utilities|Array|MakeArray "ObjectTypeQuery7") false 0 "ForOneFrame"))
        (if _returnvalue
          (for _array_element_2 _outhits
            (Utilities|Array|AddUnique (Variables|Default|GetTargetActors) (.HitActor (Collision|BreakHitResult _array_element_2))))
          (Utilities|FlowControl|DoOnce false :!label _label
            (:Completed
              (for _array_element_3 (Variables|Default|GetTargetActors)
                (bind _asbp_character (Utilities|Casting|CastToBP_Character _array_element_3))
                (Utilities|IsValid (Ability|GetAbilitySystemComponent _asbp_character)
                  (:Is%20Valid
                    (GameplayEffects|ApplyGameplayEffectToSelf :self (Ability|GetAbilitySystemComponent _asbp_character) :GameplayEffectClass "/Game/Blueprints/Effects/GE_Damage.GE_Damage_C"))))
              (Utilities|FlowControl|Delay 0.5)
              (goto _label Reset))))))))

(fn ConstructionScript
  (|CallParentFunction))