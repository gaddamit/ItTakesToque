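; Blueprint for a Brute enemy character, using a Skeleton Golem spellcast summon montage as part of its spawn sequence.
; When the spawn animation complete event fires, it plays the montage and waits for the returned duration.
; It then sets the HasSpawned blackboard key and member variable to true, signalling the AI that spawning has finished.
; The construction script only calls the parent, and the other events are disabled stubs.
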(event EventBeginPlay
  (|CallParentFunction) ; This node is disabled and will not be called.\nDrag off pins to build functionality.
)

(event Collision|EventActorBeginOverlap
  (params (OtherActor :type Actor%20Object%20Reference)))

(event EventTick
  (params (DeltaSeconds :type Float%20%28single-precision%29))
  (|CallParentFunction DeltaSeconds) ; This node is disabled and will not be called.\nDrag off pins to build functionality.
)

(event EventEventSpawnAnimationComplete
  (bind _returnvalue (Animation|PlayAnimMontage "/Game/Animations/Enemies/AM_Skeleton_Golem_Anim_Spellcast_Summon.AM_Skeleton_Golem_Anim_Spellcast_Summon" 1.0 "None"))
  (Utilities|FlowControl|Delay _returnvalue)
  (AI|Components|Blackboard|SetValueasBool (AI|GetBlackboard 0) (Utilities|Name|MakeLiteralName "HasSpawned") true)
  (Variables|Default|SetbHasSpawned true))

(fn ConstructionScript
  (|CallParentFunction))