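; BP_Character is a combat character with a type-colored ring indicator (removed for undead), GAS-driven health, hit and death animations.
; TraceWeaponPath sphere-traces each equipped weapon and sends itself Damage.Melee gameplay events targeting hit characters, throttled by a DoOnce and delay.
; OnDamageReceived rechecks the health attribute, then plays a hit montage or triggers death, which disables input and requests a controller respawn.
; Unpossessing destroys the character and its weapons.
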(event Custom|OnDeath
  (Input|DisableInput 0)
  (bind _returnvalue (Animation|PlayAnimMontage (Variables|Default|GetAnimationOnDeath) 1.0 "None"))
  (Utilities|FlowControl|Delay _returnvalue)
  (bind _aspc_custom_controller (Utilities|Casting|CastToPC_CustomController (Pawn|GetController self)))
  (Default|RespawnPlayer _aspc_custom_controller 5.0))

(event EventBeginPlay
  (if (Utilities|Enum|Equal(Enum) (Variables|Default|GetCharacterType) "UNDEAD")
    (Components|DestroyComponent (Variables|Default|GetIndicator))
    (else
      (Niagara|SetNiagaraVariable(LinearColor) (Variables|Default|GetIndicator) "User.Ring Color" (.Value (Utilities|Map|Find (.colors (Utilities|Struct|MakeS_CharacterColors "((KNIGHT, (R=1.000000,G=1.000000,B=1.000000,A=1.000000)),(BARBARIAN, (R=8.000000,G=5.000000,B=0.100000,A=1.000000)),(ROGUE, (R=8.000000,G=0.080000,B=0.200000,A=1.000000)),(MAGE, (R=1.000000,G=0.300000,B=8.000000,A=1.000000)),(NONE, (R=0.000000,G=0.000000,B=0.000000,A=0.000000)))")) (Variables|Default|GetCharacterType)))))))

(event EventOnDamageReceived
  (if (Variables|Default|GetbIsAlive)
    (Default|CallEDonDamageReceived)
    (bind _isalive (CallFunction|IsAlive))
    (bind _output_get (Variables|Default|SetbIsAlive _isalive))
    (if _output_get
      (Animation|PlayAnimMontage (Variables|Default|GetAnimationOnHit) 1.0 "None")
      (else
        (CallFunction|OnDeath)))))

(event EventUnpossessed
  (params (OldController :type Controller%20Object%20Reference))
  (CallFunction|DestroyActorandComponents))

(event EventTraceWeaponPath
  (bind _characterweapons1 (Variables|Default|GetCharacterWeapons1))
  (Utilities|Array|Clear (Variables|Default|GetTargetActors))
  (Utilities|IsValid _characterweapons1
    (:Is%20Valid
      (bind _values (Utilities|Map|Values (Variables|/Script/ItTakesToque.CharacterWeapons|GetEquippedWeapons _characterweapons1)))
      (for _array_element _values
        (bind (_outhits _returnvalue) (Collision|MultiSphereTraceForObjects (Transformation|GetWorldLocation (Variables|/Script/ItTakesToque.Weapon|GetStart _array_element)) (Transformation|GetWorldLocation (Variables|/Script/ItTakesToque.Weapon|GetEnd _array_element)) 1e+02 (Utilities|Array|MakeArray "ObjectTypeQuery8") false 0 "ForOneFrame"))
        (if _returnvalue
          (for _array_element_2 _outhits
            (Utilities|Array|AddUnique (Variables|Default|GetTargetActors) (.HitActor (Collision|BreakHitResult _array_element_2))))
          (Utilities|FlowControl|DoOnce false :!label _label
            (:Completed
              (CallFunction|SendDamageEventtoTargets (Variables|Default|GetTargetActors))
              (Utilities|FlowControl|Delay 0.5)
              (goto _label Reset))))))))

(fn ConstructionScript)

(fn SendDamageEventtoTargets
  (params (Actors :type Array%20of%20Actor%20Object%20References))
  (bind _self self)
  (for _array_element Actors
    (bind _asbp_character (Utilities|Casting|CastToBP_Character _array_element))
    (Ability|SendGameplayEventtoActor _self "(TagName=\"Damage.Melee\")" (Utilities|Struct|MakeGameplayEventData "(TagName=\"\")" _self _asbp_character 0 0 "()" (GameplayTags|GetOwnedGameplayTags 0 :!class /Script/GameplayTags.BlueprintGameplayTagLibrary) (GameplayTags|GetOwnedGameplayTags _asbp_character :!class /Script/GameplayTags.BlueprintGameplayTagLibrary) 0.0 (Ability|TargetData|AbilityTargetDatafromActor _asbp_character)))))

(fn DestroyActorandComponents
  (bind _characterweapons1 (Variables|Default|GetCharacterWeapons1))
  (Utilities|IsValid _characterweapons1
    (:Is%20Valid
      (bind _values (Utilities|Map|Values (Variables|/Script/ItTakesToque.CharacterWeapons|GetEquippedWeapons _characterweapons1)))
      (for _array_element _values
        (Actor|DestroyActor _array_element))
      (Actor|DestroyActor))))

(fn GetHPPercentage
  (bind _my2abilitysystem (Variables|Default|GetMy2AbilitySystem))
  (bind (_bfound _returnvalue) (Class|AbilitySystemComponent|GetGameplayAttributeValue _my2abilitysystem "(AttributeName=\"Health\",Attribute=/Script/ItTakesToque.CharacterAttributeSet:Health,AttributeOwner=\"/Script/CoreUObject.Class'/Script/ItTakesToque.CharacterAttributeSet'\")"))
  (if _bfound
    (return (Math|Float|SafeDivide _returnvalue 1e+01))))

(fn IsAlive
  (bind _my2abilitysystem (Variables|Default|GetMy2AbilitySystem))
  (bind (_bfound _returnvalue) (Class|AbilitySystemComponent|GetGameplayAttributeValue _my2abilitysystem "(AttributeName=\"Health\",Attribute=/Script/ItTakesToque.CharacterAttributeSet:Health,AttributeOwner=\"/Script/CoreUObject.Class'/Script/ItTakesToque.CharacterAttributeSet'\")"))
  (if _bfound
    (return (> _returnvalue 0.0))
    (else
      (return false))))