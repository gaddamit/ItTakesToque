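; PC_CustomController is a player controller that handles pawn possession, respawning and character switching.
; On possess it enables input and binds the pawn's death delegate, which triggers UnPossess.
; RespawnPlayer checks CanSpawn before and after a delay, spawns the class matching CharacterType at a GM_CoOp player start, possesses it and signals completion.
; CharacterSwitched stores the new type and refreshes the UI's skill icons.
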(event Custom|RespawnPlayer
  (params (Duration :type Float%20%28double-precision%29))
  (if (Variables|Respawn|GetCanSpawn)
    (Default|CallPlayerRespawnStarted Duration)
    (Utilities|FlowControl|Delay Duration)
    (if (Variables|Respawn|GetCanSpawn)
      (bind _asgm_co_op (Utilities|Casting|CastToGM_CoOp (Game|GetGameMode)))
      (bind _newpawn (CallFunction|CreatePawn (Variables|Default|GetCharacterType) (Class|GameModeBase|FindPlayerStart _asgm_co_op self)))
      (Pawn|Possess _newpawn)
      (Variables|Respawn|SetIsRespawnComplete true)
      (Default|CallPlayerRespawnCompleted))))

(event Custom|Character%20Switched
  (params (CharacterType :type ECharacterType%20Enum :default "NONE"))
  (Variables|Default|SetCharacterType CharacterType)
  (bind _asui_player_base (Utilities|Casting|CastToUI_Player_Base (Variables|UI|GetUIWidget)))
  (Default|UpdateSkillIcons _asui_player_base))

(event Custom|OnPawnDeath
  (Pawn|UnPossess))

(event EventBeginPlay)

(event EventTick
  (params (DeltaSeconds :type Float%20%28single-precision%29)))

(event EventPossess
  (params (PossessedPawn :type Pawn%20Object%20Reference))
  (bind _asbp_character (Utilities|Casting|CastToBP_Character PossessedPawn))
  (EventDispatchers|BindEventtoEDonDeath _asbp_character (delegate Custom|OnPawnDeath))
  (Input|EnableInput _asbp_character self)
  (Default|CallPlayerPossessed)
  (Variables|Respawn|SetIsRespawnComplete false))

(fn ConstructionScript)

(fn CreatePawn
  (params (NewType :type ECharacterType%20Enum :default "NONE") (PlayerStart :type Actor%20Object%20Reference))
  (bind _returnvalue (Game|SpawnActorfromClass (Utilities|Select :Index (Variables|Default|GetCharacterType) :NONE "/Game/Blueprints/Characters/BP_Character_Knight.BP_Character_Knight_C" :KNIGHT "/Game/Blueprints/Characters/BP_Character_Knight.BP_Character_Knight_C" :BARBARIAN "/Game/Blueprints/Characters/BP_Character_Barbarian.BP_Character_Barbarian_C" :ROGUE "/Game/Blueprints/Characters/BP_Character_Rogue.BP_Character_Rogue_C" :MAGE "/Game/Blueprints/Characters/BP_Character_Mage.BP_Character_Mage_C" :UNDEAD "/Game/Blueprints/Characters/Enemies/BP_Character_Enemy_Base.BP_Character_Enemy_Base_C") (Transformation|GetActorTransform PlayerStart) "Undefined" "MultiplyWithRoot" 0 0))
  (bind _asbp_character (Utilities|Casting|CastToBP_Character _returnvalue))
  (return _asbp_character))